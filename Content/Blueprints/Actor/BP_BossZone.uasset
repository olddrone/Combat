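; BP_BossZone is a zone actor that shows a boss UI overlay while the player character is inside it.
; On BeginPlay it creates a BP_BossOverlay widget for its Boss reference, sets the boss as the widget controller and stops its Audio.
; Overlap begin and end events add or remove the overlay, only for player 0's character.
; Audio play and stop nodes are left unconnected, so zone music never starts here.
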(event EventBeginPlay
  (bind _returnvalue (UserInterface|CreateWidget "/Game/Blueprints/UI/Overlay/BP_BossOverlay.BP_BossOverlay_C" 0 (Variables|Default|GetBoss)))
  (bind _output_get (Variables|Default|SetOverlay _returnvalue))
  (Class|CBUserWidget|SetWidgetController _output_get (Variables|Default|GetBoss))
  (Audio|Components|Audio|Stop (Variables|Default|GetAudio)))

(event Collision|EventActorBeginOverlap
  (params (OtherActor :type Actor%20Object%20Reference))
  (bind _asbp_player_character (Utilities|Casting|CastToBP_PlayerCharacter (Game|GetPlayerCharacter 0)))
  (if (== _asbp_player_character OtherActor)
    (UserInterface|Viewport|AddtoViewport (Variables|Default|GetOverlay) 0)))

(event Collision|EventActorEndOverlap
  (params (OtherActor :type Actor%20Object%20Reference))
  (bind _asbp_player_character (Utilities|Casting|CastToBP_PlayerCharacter (Game|GetPlayerCharacter 0)))
  (if (== _asbp_player_character OtherActor)
    (Widget|RemovefromParent (Variables|Default|GetOverlay))))

(fn ConstructionScript)